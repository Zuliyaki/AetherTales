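; BP_Heart is a 2D health pickup that restores life to the player when touched.
; Its collision overlap accepts only BP_PlayerBase actors, adds LifeRestored to their Health clamped between zero and DefaultHealth, then calls UpdateHealth on the player.
; The heart flipbook switches to its collected animation and the actor destroys itself after a short delay.
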(event `self.Collision.OnComponentBeginOverlap`
  (params (OverlappedComponent :type "PrimitiveComponent Object Reference") (OtherActor :type "Actor Object Reference") (OtherComp :type "PrimitiveComponent Object Reference") (OtherBodyIndex :type Integer) (bFromSweep :type Boolean) (SweepResult :type "HitResult Structure (by ref)"))
  (bind _bp_playerbase (`self.BP_PlayerBase`))
  (bind _asbp_player_base (cast `/Game/0_Template2D/Blueprints/1_Player/BP_PlayerBase` OtherActor))
  (set `self.BP_PlayerBase` _asbp_player_base)
  (set `/Game/0_Template2D/Blueprints/1_Player/BP_PlayerBase.Health` (`KismetMathLibrary.FClamp` (+ (`/Game/0_Template2D/Blueprints/1_Player/BP_PlayerBase.Health` _bp_playerbase) (`self.LifeRestored`)) 0.0 (`/Game/0_Template2D/Blueprints/1_Player/BP_PlayerBase.DefaultHealth` _bp_playerbase)) _bp_playerbase)
  (`/Game/0_Template2D/Blueprints/1_Player/BP_PlayerBase.UpdateHealth` (`self.BP_PlayerBase`))
  (`PaperFlipbookComponent.SetFlipbook` (`self.Heart`) "/Game/0_Template2D/Assets/Flipbooks/PlayerFlipbook/FB_BigHeart-Collected.FB_BigHeart-Collected")
  (`KismetSystemLibrary.Delay` 0.1)
  (`self.K2_DestroyActor`))

(fn `UserConstructionScript`)