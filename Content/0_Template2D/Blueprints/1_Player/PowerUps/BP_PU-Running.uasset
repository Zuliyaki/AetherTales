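; Running power-up pickup for the 2D template player that grants a temporary speed boost.
; The first actor overlap, gated by DoOnce, hides the cube and raises PlayerRef's max walk speed.
; After a short delay it sets the speed back to a fixed value and destroys itself.
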(event `self.ReceiveActorBeginOverlap`
  (params (OtherActor :type "Actor Object Reference"))
  (`/Engine/EditorBlueprintResources/StandardMacros.DoOnce` false
    (:`Completed`
      (`SceneComponent.SetHiddenInGame` (`self.Cube`) true false)
      (set `CharacterMovementComponent.MaxWalkSpeed` 1500.0 (`Character.CharacterMovement` (`self.PlayerRef`)))
      (`KismetSystemLibrary.Delay` 3.0)
      (set `CharacterMovementComponent.MaxWalkSpeed` 700.0 (`Character.CharacterMovement` (`self.PlayerRef`)))
      (`KismetSystemLibrary.Delay` 0.0)
      (`self.K2_DestroyActor`))))

(fn `UserConstructionScript`
  (`parent.UserConstructionScript`))