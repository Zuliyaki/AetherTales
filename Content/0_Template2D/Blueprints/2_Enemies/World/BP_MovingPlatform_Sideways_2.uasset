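; A moving platform that shuttles sideways back and forth along the X axis in a 2D template game.
; Tick passes through a DoOnce into a chain of timed MoveComponentTo moves on the root, 600 units toward negative X, then back, with short pauses.
; A custom ResetMovement event reopens the DoOnce afterward, so the cycle repeats indefinitely.
; Each target is an offset from the root's current world location, fed into the relative-location input.
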(event `self.ReceiveTick`
  (params (DeltaSeconds :type "Float (single-precision)"))
  (`/Engine/EditorBlueprintResources/StandardMacros.DoOnce` false :!label _label
    (:`Completed`
      (`KismetSystemLibrary.MoveComponentTo` (`self.DefaultSceneRoot`) (+ (`SceneComponent.K2_GetComponentLocation` (`self.DefaultSceneRoot`)) (-600.0 0.0 0.0)) (struct) false false 2.0)
      (`KismetSystemLibrary.Delay` 0.5)
      (`KismetSystemLibrary.MoveComponentTo` (`self.DefaultSceneRoot`) (+ (`SceneComponent.K2_GetComponentLocation` (`self.DefaultSceneRoot`)) (600.0 0.0 -0.0)) (struct) false false 2.0)
      (`KismetSystemLibrary.Delay` 0.5)
      (`self.ResetMovement`))))

(event `ResetMovement`
  (goto _label :!via `Reset`))

(fn `UserConstructionScript`)