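; BP_Environment is a world hazard that damages the player and sends them back to a checkpoint.
; A DamageDealer hit on BP_PlayerBase stops movement, applies damage and, after a short delay, teleports the player to CheckRef.
; Input stays disabled for StunDuration while a camera fade plays.
; CheckRef is set only when BP_CheckpointReference itself hits DamageDealer, which runs the same sequence on the stored player.
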(event `self.DamageDealer.OnComponentHit`
  (params (HitComponent :type "PrimitiveComponent Object Reference") (OtherActor :type "Actor Object Reference") (OtherComp :type "PrimitiveComponent Object Reference") (NormalImpulse :type "Vector Structure") (Hit :type "HitResult Structure (by ref)"))
  ;[1 0.05673 0.1564] Damaging Player
  (`|ExecutionSequence`
    (:`then_0`
      (bind _asbp_player_base (cast `/Game/0_Template2D/Blueprints/1_Player/BP_PlayerBase` OtherActor))
      (set `self.PlayerRef` _asbp_player_base))
    (:`then_1`
      (bind _asbp_checkpoint_reference (cast `/Game/0_Template2D/Blueprints/4_References/BP_CheckpointReference` OtherActor))
      (set `self.CheckRef` _asbp_checkpoint_reference)))
  (`MovementComponent.StopMovementImmediately` (`Character.CharacterMovement` (`self.PlayerRef`)))
  (`GameplayStatics.ApplyDamage` (`self.PlayerRef`) (`self.BaseDamage`))
  (`KismetSystemLibrary.Delay` 0.5)
  (`self.K2_TeleportTo` :`self` (`self.PlayerRef`) :`DestLocation` (`self.K2_GetActorLocation` (`self.CheckRef`)))
  (`self.DisableInput` (`self.PlayerRef`) null)
  (`PlayerCameraManager.StartCameraFade` :`self` (`GameplayStatics.GetPlayerCameraManager` 0) :`FromAlpha` 1.0 :`Duration` 1.0 :`bShouldFadeAudio` true)
  (`KismetSystemLibrary.Delay` (`self.StunDuration`))
  (`self.EnableInput` (`self.PlayerRef`) null))

(fn `UserConstructionScript`)