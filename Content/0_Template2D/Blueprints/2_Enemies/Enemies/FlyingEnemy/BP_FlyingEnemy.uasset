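; Flying bee enemy Blueprint for the 2D template, built on a parent enemy class.
; The construction script copies the default health and damage values into the working health and damage variables after the parent's setup.
; On death it runs the parent logic, switches the sprite to the bee dying flipbook and turns on capsule physics simulation.
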(event `self.ReceiveBeginPlay`
  (`parent.ReceiveBeginPlay`))

(fn `EnemyDied`
  (`parent.EnemyDied`)
  (`PaperFlipbookComponent.SetFlipbook` (`self.Sprite`) "/Game/0_Template2D/Assets/Flipbooks/FlyingEnemy/FB_Bee-Dying.FB_Bee-Dying")
  (`PrimitiveComponent.SetSimulatePhysics` (`self.CapsuleComponent`) true))

(fn `UserConstructionScript`
  (`parent.UserConstructionScript`)
  (`|ExecutionSequence`
    (:`then_0`
      (set `self.EnemyHealth` (`self.EnemyDefaultHealth`)))
    (:`then_1`
      (set `self.EnemyDamage` (`self.EnemyDefaultDamage`)))))