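; Enemy projectile, filed under the Cannon enemy, that damages the player on contact.
; A sphere overlap with BP_PlayerBase applies BaseDamage and destroys the projectile, which otherwise expires after SelfDestructionTimer.
; Each tick, a short Visibility line trace along fixed world +X, independent of the projectile's facing, destroys it on a hit to detect walls.
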(event `self.ReceiveBeginPlay`
  ;[1 1 1] Destroy self
  (`KismetSystemLibrary.Delay` (`self.SelfDestructionTimer`))
  (`self.K2_DestroyActor`))

(event `self.Sphere.OnComponentBeginOverlap`
  (params (OverlappedComponent :type "PrimitiveComponent Object Reference") (OtherActor :type "Actor Object Reference") (OtherComp :type "PrimitiveComponent Object Reference") (OtherBodyIndex :type Integer) (bFromSweep :type Boolean) (SweepResult :type "HitResult Structure (by ref)"))
  ;[1 1 1] Damage Player
  (bind _asbp_player_base (cast `/Game/0_Template2D/Blueprints/1_Player/BP_PlayerBase` OtherActor))
  (bind _output_get (set `self.PlayerRef` _asbp_player_base))
  (`GameplayStatics.ApplyDamage` _output_get (`self.Base Damage`))
  (`self.K2_DestroyActor`))

(event `self.ReceiveTick`
  (params (DeltaSeconds :type "Float (single-precision)"))
  (bind _returnvalue (`self.K2_GetActorLocation`))
  ;[1 1 1] Destroy projectile when hiting wall
  (bind (_outhit _returnvalue_2) (`KismetSystemLibrary.LineTraceSingle` _returnvalue (+ _returnvalue (10.0 0.0 0.0)) "TraceTypeQuery1"))
  (if _returnvalue_2
    (`self.K2_DestroyActor`)))

(fn `UserConstructionScript`)