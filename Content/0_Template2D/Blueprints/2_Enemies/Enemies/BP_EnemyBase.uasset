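; Base enemy Blueprint for a 2D game template, handling contact damage to the player, its own health and death.
; The construction script seeds health and damage from defaults, and capsule hits on BP_PlayerBase apply that damage.
; Incoming damage lowers clamped health and triggers a one-time death that ignores two custom collision channels, disables overlaps, stops sprite looping and detaches the controller.
; UpdateEnemyHealth is an empty stub.
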(event `self.CapsuleComponent.OnComponentHit`
  (params (HitComponent :type "PrimitiveComponent Object Reference") (OtherActor :type "Actor Object Reference") (OtherComp :type "PrimitiveComponent Object Reference") (NormalImpulse :type "Vector Structure") (Hit :type "HitResult Structure (by ref)"))
  ;[0.2235 1 0.3569] Damaging Player
  (bind _asbp_player_base (cast `/Game/0_Template2D/Blueprints/1_Player/BP_PlayerBase` OtherActor))
  (set `self.PlayerRef` _asbp_player_base)
  (`GameplayStatics.ApplyDamage` (`self.PlayerRef`) (`self.EnemyDamage`))
  (set `self.HittingPlayer` true)
  (`KismetSystemLibrary.Delay` 0.2))

(event `self.ReceiveAnyDamage`
  (params (Damage :type "Float (single-precision)") (DamageType :type "DamageType Object Reference") (InstigatedBy :type "Controller Object Reference") (DamageCauser :type "Actor Object Reference"))
  ;[0.2232 1 0.3564] Any Damage System
  (`|ExecutionSequence`
    (:`then_0`
      (set `self.EnemyHealth` (`KismetMathLibrary.FClamp` (- (`self.EnemyHealth`) Damage) 0.0 (`self.EnemyDefaultHealth`)))
      (if (and (<= (`self.EnemyHealth`) 0.0) (not (`self.IsDead`)))
        (set `self.IsDead` true)
        (`self.EnemyDied`)))
    (:`then_1`
      (`KismetSystemLibrary.Delay` 0.0))))

(fn `EnemyDied`
  ;[1 0 0.06996] Enemy Died
  (`PrimitiveComponent.SetCollisionResponseToChannel` (`self.CapsuleComponent`) "ECC_GameTraceChannel2" "ECR_Ignore")
  (`PrimitiveComponent.SetCollisionResponseToChannel` (`self.CapsuleComponent`) "ECC_GameTraceChannel3" "ECR_Ignore")
  (`PaperFlipbookComponent.SetLooping` (`self.Sprite`) false)
  (set `PrimitiveComponent.bGenerateOverlapEvents` false (`self.CapsuleComponent`))
  (`self.DetachFromControllerPendingDestroy`))

(fn `UpdateEnemyHealth`)

(fn `UserConstructionScript`
  (`|ExecutionSequence`
    (:`then_0`
      (set `self.EnemyHealth` (`self.EnemyDefaultHealth`)))
    (:`then_1`
      (set `self.EnemyDamage` (`self.EnemyDefaultDamage`)))))